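; BP_Door is a door actor that swings open when an actor tagged "Player" enters its Sphere and swings back when that actor leaves.
; Two timelines add or subtract their track value from SMDoor's current world yaw on each update, zeroing roll and pitch.
; Opening stops past a fixed world yaw of 90 degrees, while closing stops below DefRot, which is captured on every ActorBeginOverlap rather than at BeginPlay.
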(event `self.ReceiveActorBeginOverlap`
  (params (OtherActor :type "Actor Object Reference"))
  (set `self.Def_Rot` (`SceneComponent.K2_GetComponentRotation` (`self.SM_Door`))))

(event `self.Sphere.OnComponentBeginOverlap`
  (params (OverlappedComponent :type "PrimitiveComponent Object Reference") (OtherActor :type "Actor Object Reference") (OtherComp :type "PrimitiveComponent Object Reference") (OtherBodyIndex :type Integer) (bFromSweep :type Boolean) (SweepResult :type "HitResult Structure (by ref)"))
  (bind (_returnvalue_roll _returnvalue_pitch _returnvalue_yaw) (`KismetMathLibrary.BreakRotator` (`SceneComponent.K2_GetComponentRotation` (`self.SM_Door`))))
  (if (`self.ActorHasTag` OtherActor "Player")
    (bind (_direction `_新規track_0`) (`Timeline|タイムライン_0` :!label _label)
      (:`Update`
        (if (<= _returnvalue_yaw 90.0)
          (`SceneComponent.K2_SetWorldRotation` (`self.SM_Door`) (`KismetMathLibrary.MakeRotator` 0.0 0.0 (+ _returnvalue_yaw `_新規track_0`)) false false)
          (else
            (goto _label :!via `Stop`)))))))

(event `self.Sphere.OnComponentEndOverlap`
  (params (OverlappedComponent :type "PrimitiveComponent Object Reference") (OtherActor :type "Actor Object Reference") (OtherComp :type "PrimitiveComponent Object Reference") (OtherBodyIndex :type Integer))
  (bind (_def_rot_roll _def_rot_pitch _def_rot_yaw) (`KismetMathLibrary.BreakRotator` (`self.Def_Rot`)))
  (bind (_returnvalue_roll _returnvalue_pitch _returnvalue_yaw) (`KismetMathLibrary.BreakRotator` (`SceneComponent.K2_GetComponentRotation` (`self.SM_Door`))))
  (if (`self.ActorHasTag` OtherActor "Player")
    (bind (_direction `_新規track_0`) (`Timeline|タイムライン_1` :!label _label_2)
      (:`Update`
        (if (>= _returnvalue_yaw _def_rot_yaw)
          (`SceneComponent.K2_SetWorldRotation` (`self.SM_Door`) (`KismetMathLibrary.MakeRotator` 0.0 0.0 (- _returnvalue_yaw `_新規track_0`)) false false)
          (else
            (goto _label_2 :!via `Stop`)))))))

(fn `UserConstructionScript`)