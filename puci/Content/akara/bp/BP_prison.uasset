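; BP_prison is a prison mesh that rises and lowers in response to lever events.
; Lever on and off events set direction flags and play a shared timeline.
; Each timeline update moves the mesh vertically by the track value, used as a step rather than an absolute position.
; The timeline stops once the mesh passes its upper offset or returns to its starting height recorded at BeginPlay.
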(event `self.ReceiveBeginPlay`
  (set `self.StartPos` (`SceneComponent.K2_GetComponentLocation` (`self.SM_prison`))))

(event `self.event_Lever.Lever_On`
  (bind (_startpos_x _startpos_y _startpos_z) (`KismetMathLibrary.BreakVector` (`self.StartPos`)))
  (bind (_startpos_x_2 _startpos_y_2 _startpos_z_2) (`KismetMathLibrary.BreakVector` (`self.StartPos`)))
  (bind (_returnvalue_x _returnvalue_y _returnvalue_z) (`KismetMathLibrary.BreakVector` (`SceneComponent.K2_GetComponentLocation` (`self.SM_prison`))))
  (set `self.isDown` false)
  (set `self.isUp` true)
  (bind (_direction `_新規track_0`) (`Timeline|Up_Down_Value` :!label _label)
    (:`Update`
      (if (`self.isUp`)
        (if (<= _returnvalue_z (+ (`self.UpZMax`) _startpos_z_2))
          (`SceneComponent.K2_SetWorldLocation` (`self.SM_prison`) (`KismetMathLibrary.MakeVector` _returnvalue_x _returnvalue_y (+ _returnvalue_z `_新規track_0`)) false false)
          (else
            (set `self.isUp` false)
            (goto _label :!via `Stop`)))
        (elif (>= _returnvalue_z _startpos_z)
          (`SceneComponent.K2_SetWorldLocation` (`self.SM_prison`) (`KismetMathLibrary.MakeVector` _returnvalue_x _returnvalue_y (- _returnvalue_z `_新規track_0`)) false false)
          (else
            (set `self.isDown` false)
            (goto _label :!via `Stop`)))))))

(event `self.event_Lever.Lever_Off`
  (set `self.isUp` false)
  (set `self.isDown` true)
  (goto _label))

(fn `UserConstructionScript`)