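; BP_Lever is an interactable lever that the player toggles with E while inside its sphere trigger, which enables and disables input.
; The Lever timeline adds or subtracts its RotValue from the mesh's world roll each update until it passes the on or off limit.
; It then flips IsOn and calls the LeverOn or LeverOff dispatcher, with IsWorking blocking presses mid-swing.
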(event `self.ReceiveBeginPlay`
  (set `self.Off_rot` -30.0)
  (set `self.On_rot` 30.0)
  (set `self.isOn` false)
  (set `self.isWorking` false))

(event `Key|E`
  (params (Key :type "Key Structure"))
  (bind (_returnvalue_roll _returnvalue_pitch _returnvalue_yaw) (`KismetMathLibrary.BreakRotator` (`SceneComponent.K2_GetComponentRotation` (`self.SM_Lever1`))))
  (bind (_returnvalue_roll_2 _returnvalue_pitch_2 _returnvalue_yaw_2) (`KismetMathLibrary.BreakRotator` (`SceneComponent.K2_GetComponentRotation` (`self.SM_Lever1`))))
  (:`Pressed`
    (if (not (`self.isWorking`))
      (set `self.isWorking` true)
      (bind (_direction _rotvalue) (`Timeline|lever`)
        (:`Update`
          (if (`self.isWorking`)
            (if (`self.isOn`)
              (if (>= (`self.Off_rot`) _returnvalue_roll_2)
                (set `self.isOn` false)
                (set `self.isWorking` false)
                (`self.Lever_Off`)
                (else
                  (`SceneComponent.K2_SetWorldRotation` (`self.SM_Lever1`) (`KismetMathLibrary.MakeRotator` (- _returnvalue_roll_2 _rotvalue) _returnvalue_pitch_2 _returnvalue_yaw_2) false false)))
              (elif (>= _returnvalue_roll (`self.On_rot`))
                (set `self.isOn` true)
                (set `self.isWorking` false)
                (`self.Lever_On`)
                (add `self.Lever_On` (delegate `Lever_On_Event`))
                (else
                  (`SceneComponent.K2_SetWorldRotation` (`self.SM_Lever1`) (`KismetMathLibrary.MakeRotator` (+ _returnvalue_roll _rotvalue) _returnvalue_pitch _returnvalue_yaw) false false))))))))))

(event `Lever_On_Event`)

(event `self.Sphere.OnComponentBeginOverlap`
  (params (OverlappedComponent :type "PrimitiveComponent Object Reference") (OtherActor :type "Actor Object Reference") (OtherComp :type "PrimitiveComponent Object Reference") (OtherBodyIndex :type Integer) (bFromSweep :type Boolean) (SweepResult :type "HitResult Structure (by ref)"))
  (if (`self.ActorHasTag` OtherActor "Player")
    (`self.EnableInput` (`GameplayStatics.GetPlayerController` 0))))

(event `self.Sphere.OnComponentEndOverlap`
  (params (OverlappedComponent :type "PrimitiveComponent Object Reference") (OtherActor :type "Actor Object Reference") (OtherComp :type "PrimitiveComponent Object Reference") (OtherBodyIndex :type Integer))
  (if (`self.ActorHasTag` OtherActor "Player")
    (`self.DisableInput` (`GameplayStatics.GetPlayerController` 0))))

(fn `UserConstructionScript`)